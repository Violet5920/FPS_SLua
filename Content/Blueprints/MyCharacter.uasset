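; Player character Blueprint that hands movement, look and jump input to Lua script and fights with a spawned weapon.
; On BeginPlay it spawns a test weapon at its own transform, stores it as the current weapon and equips it.
; Axis and jump inputs call named Lua member functions, while Fire press and release start and stop the weapon's attack directly.
; Native movement and Lua fire nodes remain unconnected.
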(event `self.ReceiveBeginPlay`
  (bind _returnvalue (`|SpawnActorFromClass` "/Game/Blueprints/Weapon_Test.Weapon_Test_C" (`self.GetTransform`) "AlwaysSpawn" "OverrideRootScale" null null))
  (bind _output_get (set `self.CurrentWeapon` _returnvalue))
  (`WeaponBase.Equip` _output_get self))

(event `InputAxis|MoveForward`
  (params (AxisValue :type "Float (single-precision)"))
  (bind _returnvalue (`LuaBlueprintLibrary.CreateVarFromNumber` AxisValue))
  (`self.CallLuaMember` "MoveForward" (`|MakeArray` _returnvalue)))

(event `InputAxis|MoveRight`
  (params (AxisValue :type "Float (single-precision)"))
  (bind _returnvalue (`LuaBlueprintLibrary.CreateVarFromNumber` AxisValue))
  (`self.CallLuaMember` "MoveRight" (`|MakeArray` _returnvalue)))

(event `InputAxis|Lookup`
  (params (AxisValue :type "Float (single-precision)"))
  (bind _returnvalue (`LuaBlueprintLibrary.CreateVarFromNumber` AxisValue))
  (`self.CallLuaMember` "Lookup" (`|MakeArray` _returnvalue)))

(event `InputAxis|Turn`
  (params (AxisValue :type "Float (single-precision)"))
  (bind _returnvalue (`LuaBlueprintLibrary.CreateVarFromNumber` AxisValue))
  (`self.CallLuaMember` "Turn" (`|MakeArray` _returnvalue)))

(event `InputAction|Jump`
  (params (Key :type "Key Structure"))
  (bind _array (`|MakeArray`))
  (:`Pressed`
    (`self.CallLuaMember` "OnJumpStart" _array))
  (:`Released`
    (`self.CallLuaMember` "OnJumpEnd" _array)))

(event `InputAction|Fire`
  (params (Key :type "Key Structure"))
  (bind _currentweapon (`self.CurrentWeapon`))
  (:`Pressed`
    (`WeaponBase.StartAttack` _currentweapon))
  (:`Released`
    (`WeaponBase.StopAttack` _currentweapon)))

(fn `UserConstructionScript`)